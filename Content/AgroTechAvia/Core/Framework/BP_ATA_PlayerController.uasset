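; Player controller for AgroTechAvia that drives camera view targets and input mode as lessons and parts change.
; On BeginPlay it caches a level CameraActor as the main menu camera and binds to WidgetControllerSubsystem lesson, part-focus and view-target events.
; Lesson activation and deactivation toggle input mode, while deactivation or unselection returns to the menu camera.
; View changes blend under a timer, queuing only the latest request made mid-blend until the blend ends.
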(event `self.ReceiveBeginPlay`
  (`parent.ReceiveBeginPlay`)
  (`self.SetUpReferences`)
  (`self.SetUpBinds`))

(fn `CameraBlendEnded`
  (bind _newviewtarget (`self.NewViewTarget`))
  (`KismetSystemLibrary.K2_ClearAndInvalidateTimerHandle` (`self.CameraBlendTimer`))
  (`/Engine/EditorBlueprintResources/StandardMacros.IsValid` _newviewtarget
    (:`Is Valid`
      (`self.ChangeViewTarget` _newviewtarget))))

(fn `ChangeViewTarget`
  (params (NewViewTarget :type "Actor Object Reference"))
  (bind _blendtime (`self.BlendTime`))
  (if (`KismetSystemLibrary.K2_IsValidTimerHandle` (`self.CameraBlendTimer`))
    (set `self.NewViewTarget` NewViewTarget)
    (else
      (set `self.NewViewTarget` null)
      (`self.SetViewTargetWithBlend` NewViewTarget _blendtime)
      (bind _returnvalue (`KismetSystemLibrary.K2_SetTimerDelegate` (`|CreateDelegate` :!event `CameraBlendEnded`) _blendtime))
      (set `self.CameraBlendTimer` _returnvalue))))

(fn `HandleOnLessonActivated`
  (params (StudyObjectTag :type "GameplayTag Structure"))
  (`self.ToggleInputMode` false))

(fn `HandleOnLessonDeactivated`
  (`self.ChangeViewTarget` (`self.MainMenuCamera`))
  (`self.ToggleInputMode` true))

(fn `HandleOnLessonUnselected`
  (`self.ChangeViewTarget` (`self.MainMenuCamera`)))

(fn `HandleOnPartFocused`
  (params (Actor :type "Actor Object Reference") (PartTag :type "GameplayTag Structure"))
  (`self.ChangeViewTarget` Actor))

(fn `HandleOnViewTargetChanged`
  (params (Actor :type "Actor Object Reference"))
  (`self.ChangeViewTarget` Actor))

(fn `SetUpBinds`
  (bind _returnvalue (subsystem `WidgetControllerSubsystem`))
  (add `WidgetControllerSubsystem.OnLessonDeactivated` _returnvalue (`|CreateDelegate` :!event `HandleOnLessonDeactivated`))
  (add `WidgetControllerSubsystem.OnPartFocused` _returnvalue (`|CreateDelegate` :!event `HandleOnPartFocused`))
  (add `WidgetControllerSubsystem.OnViewTargetChanged` _returnvalue (`|CreateDelegate` :!event `HandleOnViewTargetChanged`))
  (add `WidgetControllerSubsystem.OnLessonActivated` _returnvalue (`|CreateDelegate` :!event `HandleOnLessonActivated`))
  (add `WidgetControllerSubsystem.OnLessonDeactivated` _returnvalue (`|CreateDelegate` :!event `HandleOnLessonUnselected`))
  (add `WidgetControllerSubsystem.OnLessonUnselected` _returnvalue (`|CreateDelegate` :!event `HandleOnLessonUnselected`)))

(fn `SetUpReferences`
  (bind _returnvalue (`GameplayStatics.GetActorOfClass` "/Script/Engine.CameraActor"))
  (set `self.MainMenuCamera` _returnvalue))

(fn `UserConstructionScript`)