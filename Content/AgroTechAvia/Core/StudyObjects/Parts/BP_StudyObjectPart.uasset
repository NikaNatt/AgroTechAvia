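; BP_StudyObjectPart is a selectable part of a study object, identified by a PartTag and paired with its own camera.
; When selected, it reports the tag to the WidgetControllerSubsystem as the focused part.
; Its construction script positions, rotates and scales the ATACamera child actor component from per-part settings, then copies PartTag into the spawned BP_ATA_Camera's CameraTag, so part and camera share one identifier.
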(event `StudyObjectInterface.OnObjectSelected`
  (`WidgetControllerSubsystem.OnPartFocused` (subsystem `WidgetControllerSubsystem`) (`self.PartTag`)))

(fn `UserConstructionScript`
  (bind _atacamera (`self.ATACamera`))
  (`SceneComponent.K2_SetRelativeRotation` _atacamera (`self.CameraRotation`) false false)
  (`SceneComponent.K2_SetRelativeLocation` _atacamera (`self.CameraLocation`) false false)
  (`SceneComponent.SetWorldScale3D` _atacamera (0.4 0.4 0.4))
  (bind _asbp_ata_camera (cast `/Game/AgroTechAvia/Core/BP_ATA_Camera` (`ChildActorComponent.ChildActor` (`self.ATACamera`))))
  (set `/Game/AgroTechAvia/Core/BP_ATA_Camera.CameraTag` (`self.PartTag`) _asbp_ata_camera))